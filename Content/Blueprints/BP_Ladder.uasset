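; BP_Ladder is a ladder actor with configurable height and rung spacing that tells overlapping actors when they are at it.
; Initialize, run in construction and on BeginPlay, positions LadderTop, stretches both sides and the collider to match, and rebuilds rungs as mesh instances every BarGap.
; The collider sends SetLadderMessage to the overlapping actor, passing itself on begin overlap and no ladder on end overlap.
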(event OnComponentBeginOverlap(Collider)
  (params (OverlappedComponent :type Primitive%20Component%20Object%20Reference) (OtherActor :type Actor%20Object%20Reference) (OtherComp :type Primitive%20Component%20Object%20Reference) (OtherBodyIndex :type Integer) (bFromSweep :type Boolean) (SweepResult :type Hit%20Result%20Structure%20%28by%20ref%29))
  (Class|BPIClimb|SetLadder(Message) OtherActor self))

(event OnComponentEndOverlap(Collider)
  (params (OverlappedComponent :type Primitive%20Component%20Object%20Reference) (OtherActor :type Actor%20Object%20Reference) (OtherComp :type Primitive%20Component%20Object%20Reference) (OtherBodyIndex :type Integer))
  (Class|BPIClimb|SetLadder(Message) OtherActor))

(event Custom|Initialize
  (bind _right (Variables|Default|GetRight))
  (bind _collider (Variables|Default|GetCollider))
  (bind _bar (Variables|Default|GetBar))
  (bind _left (Variables|Default|GetLeft))
  (Transformation|SetRelativeLocation (Variables|Default|GetLadderTop) (Math|Vector|MakeVector 0.0 0.0 (Variables|Default|GetHeight)) false false)
  (Utilities|Conversion _left _left)
  (Utilities|Conversion _right _right)
  (Utilities|Conversion _collider _collider)
  (Variables|Default|Settemp_Height 0.0)
  (Components|InstancedStaticMesh|ClearInstances _bar)
  (while (< (Variables|Default|Gettemp_Height) (.z (Variables|/Script/Engine.SceneComponent|GetRelativeLocation (Variables|Default|GetLadderTop))))
    (Components|InstancedStaticMesh|AddInstance _bar (Math|Transform|MakeTransform (Math|Vector|MakeVector 0.0 0.0 (Variables|Default|Gettemp_Height)) "0, 0, 0" "0.075000,0.850000,0.050000") false)
    (Variables|Default|Settemp_Height (+ (Variables|Default|Gettemp_Height) (Variables|Default|GetBarGap)))))

(event EventBeginPlay
  (CallFunction|Initialize))

(event Collision|EventActorBeginOverlap
  (params (OtherActor :type Actor%20Object%20Reference)))

(event EventTick
  (params (DeltaSeconds :type Float%20%28single-precision%29)))

(fn ConstructionScript
  (CallFunction|Initialize))